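; Game mode for the patching stage that monitors content patch progress and opens L_PatchGameLevel once it completes.
; TootStart, not called by this graph's live logic, calls PatchGame on BP_CDGameInst and stores the result as the in-progress flag.
; While that flag is set, Tick polls the game instance's download and mount percentages, prints them, and travels when both reach 100.
; Retry-counter and delay nodes are left disconnected.
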(event `self.ReceiveBeginPlay`
  (`KismetSystemLibrary.PrintString` "Game mode begin......."))

(event `self.ReceiveTick`
  (params (DeltaSeconds :type "Float (single-precision)"))
  (`self.TootTick`))

(event `TootStart`
  (bind _asbp_cdgame_inst (cast `/Game/PatchGame/BP_CDGameInst` (`GameplayStatics.GetGameInstance`)))
  (bind _output_get (set `self.CurrGameInst` _asbp_cdgame_inst))
  (bind _returnvalue (`MainGameInst.PatchGame` _output_get))
  (bind _output_get_2 (set `self.IsPatchingInProgress` _returnvalue))
  (if _output_get_2
    (`KismetSystemLibrary.PrintString` "Patch game in progress.......")
    (else
      (`KismetSystemLibrary.PrintString` "Patch game failed......."))))

(event `TootTick`
  (bind (_bytesdownloaded _totalbytes _downloadpercent _chunkmounted _totalchunktomount _mountpercent) (`MainGameInst.FireLoadingProgress` (`self.CurrGameInst`)))
  (if (`self.IsPatchingInProgress`)
    (`KismetSystemLibrary.PrintString` (`KismetStringLibrary.BuildString_Double` "" "Curr Loading Progress : " _downloadpercent "%") true true (struct :`G` 0.66 :`B` 1.0 :`A` 1.0) 2.0 "LoadP")
    (`KismetSystemLibrary.PrintString` (`KismetStringLibrary.BuildString_Double` "" "Curr Mounting Progress : " _mountpercent "%") true true (struct :`G` 0.66 :`B` 1.0 :`A` 1.0) 2.0 "MountP")
    (if (and (>= _downloadpercent 100.0) (>= _mountpercent 100.0))
      (`GameplayStatics.OpenLevel` "L_PatchGameLevel")
      (`KismetSystemLibrary.PrintString` "got to .........   L_PatchGameLevel"))))

(fn `UserConstructionScript`)